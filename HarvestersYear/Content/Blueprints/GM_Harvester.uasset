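; Game mode for the Harvester game that sets up the HUD, main camera and a timed scoring round.
; BeginPlay loads or creates the high-score save, then starts a looping timer that decrements the remaining time.
; AddScore overwrites the current score rather than accumulating it.
; EndRound saves to two separate slots after a delay if the high score is beaten, but its timer-expiry trigger is unwired, as is storing the HUD reference.
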(event `self.ReceiveBeginPlay`
  ; Set Up & Initialization
  (`KismetSystemLibrary.Delay` 0.2)
  (`self.LoadGame`)
  (bind _returnvalue (`|CreateWidget` "/Game/Blueprints/WBP_GameHUD.WBP_GameHUD_C"))
  (`UserWidget.AddToViewport` _returnvalue 0)
  (bind _outactors (`GameplayStatics.GetAllActorsWithTag` "MainCamera"))
  (`PlayerController.SetViewTargetWithBlend` (`GameplayStatics.GetPlayerController` 0) (`|GetArrayItem` _outactors) 0.0 "VTBlend_Linear" 0.0 false)
  (set `self.RoundDuration` 75)
  (`self.StartRound`))

(event `LoadGame`
  ; Set Up & Initialization
  (`GameplayStatics.DoesSaveGameExist` "HighScoreSave")
  (if true
    (bind _returnvalue (`GameplayStatics.LoadGameFromSlot` "HighScoreSave"))
    (bind _assg_high_scores (cast `/Game/Blueprints/SG_HighScores` _returnvalue))
    (set `self.SaveGameRef` _assg_high_scores)
    (else
      (bind _returnvalue_2 (`GameplayStatics.CreateSaveGameObject` "/Game/Blueprints/SG_HighScores.SG_HighScores_C"))
      (set `self.SaveGameRef` _returnvalue_2))))

(event `SaveGame`
  ; Set Up & Initialization
  (`GameplayStatics.SaveGameToSlot` (`self.SaveGameRef`) "HighScoreSave"))

(event `StartRound`
  ; Round Management
  (set `self.TimeRemaining` (`self.RoundDuration`))
  (`self.UpdateTimer`)
  (`KismetSystemLibrary.K2_SetTimer` null "UpdateTimer" 1.0 true))

(event `/Game/Blueprints/BI_GameEvents.AddScore`
  (params (PointsToAdd :type Integer))
  ; Update the Score
  (set `self.CurrentScore` PointsToAdd))

(event `EndRound`
  ; Round Management
  (`KismetSystemLibrary.Delay` 15.0)
  (if (> (`self.CurrentScore`) (`self.HighScore`))
    (`self.SaveGame`)
    (bind _returnvalue (`GameplayStatics.CreateSaveGameObject` "/Game/Blueprints/BP_HarvesterSave.BP_HarvesterSave_C"))
    (`GameplayStatics.SaveGameToSlot` _returnvalue "HighScoreSlot")))

(fn `UpdateTimer`
  (bind _output_get (set `self.TimeRemaining` (- (`self.TimeRemaining`) 1))))

(fn `UserConstructionScript`)